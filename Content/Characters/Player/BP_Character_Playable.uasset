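; BP_Character_Playable is the player character Blueprint, providing basic movement and mouse look.
; MoveForward and MoveRight axis inputs add movement along the actor's forward and right vectors.
; MouseX and MouseY feed controller yaw and pitch directly, without scaling.
; BeginPlay and overlap events are disabled stubs, and the construction script only calls its parent.
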(event `InputAxis|MoveForward`
  (params (AxisValue :type "Float (single-precision)"))
  (`self.AddMovementInput` (`self.GetActorForwardVector`) AxisValue))

(event `InputAxis|MouseX`
  (params (AxisValue :type "Float (single-precision)"))
  (`self.AddControllerYawInput` AxisValue))

(event `InputAxis|MoveRight`
  (params (AxisValue :type "Float (single-precision)"))
  (`self.AddMovementInput` (`self.GetActorRightVector`) AxisValue))

(event `InputAxis|MouseY`
  (params (AxisValue :type "Float (single-precision)"))
  (`self.AddControllerPitchInput` AxisValue))

(fn `UserConstructionScript`
  (`parent.UserConstructionScript`))