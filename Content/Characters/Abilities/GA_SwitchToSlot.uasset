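; Gameplay ability that switches a Gladiator character's equipment to the next item in a target slot.
; On activation it asks the owning character for the next item in SlotToTarget, without falling back to the first, and equips it if valid.
; The ability ends immediately after this check, so it holds no ongoing state.
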(event `self.K2_ActivateAbility`
  (`self.HandleAbility`)
  (`self.K2_EndAbility`))

(fn `HandleAbility`
  (locals (LocalItem :type "ItemEquipable Object Reference"))
  (bind _asgladiator_character (cast `GladiatorCharacter` (`self.GetOwningActorFromActorInfo`)))
  (bind _returnvalue (`GladiatorCharacter.GetNextItemInSlot` _asgladiator_character (`self.SlotToTarget`) false))
  (bind _output_get (set `local.LocalItem` _returnvalue))
  (`/Engine/EditorBlueprintResources/StandardMacros.IsValid` _output_get
    (:`Is Valid`
      (`GladiatorCharacter.EquipItem` _asgladiator_character (`local.LocalItem`)))))