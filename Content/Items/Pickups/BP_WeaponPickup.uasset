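; BP_WeaponPickup is a pickup that grants its configured ItemClass to the user's InventoryComponent, skipping users who already hold that class.
; The construction script previews the item by copying the class default Mesh1PAsset onto the Mesh3P skeletal mesh.
; On BeginPlay, an invalid ItemClass prints an error and disables the actor's collision.
; BlueprintCanPickup always returns true, so the duplicate check happens only when the pickup is handled.
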(event `self.ReceiveBeginPlay`
  (if (not (`KismetSystemLibrary.IsValidClass` (`self.ItemClass`)))
    (`KismetSystemLibrary.PrintString` (`KismetStringLibrary.Concat_StrStr` "ERROR: " (`KismetSystemLibrary.GetDisplayName` self) " will not spawn its pickup class because the WeaponToAdd class is invalid. Please add a class for this to use!") false)
    (`self.SetActorEnableCollision` false)))

(event `self.BlueprintHandlePickup`
  (params (ForUser :type "GladiatorCharacter Object Reference"))
  (bind _inventorycomponent (`GladiatorCharacter.InventoryComponent` ForUser))
  (if (not (`InventoryComponent.HasItemClassInInventory` _inventorycomponent (`self.ItemClass`)))
    (`InventoryComponent.GiveItemClass` _inventorycomponent (`self.ItemClass`))))

(fn `BlueprintCanPickup`
  (params (ForUser :type "GladiatorCharacter Object Reference"))
  (returns (ReturnValue :type Boolean))
  (return true))

(fn `UserConstructionScript`
  (if (`KismetSystemLibrary.IsValidClass` (`self.ItemClass`))
    (`SkinnedMeshComponent.SetSkinnedAssetAndUpdate` (`self.Mesh3P`) (`.Mesh1PAsset` (defaults `Object` (`self.ItemClass`))) true)))