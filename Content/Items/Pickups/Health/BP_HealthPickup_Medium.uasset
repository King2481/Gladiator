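; Medium health pickup Blueprint that restores health to the character that collects it.
; It extends a parent pickup class, adding a condition that the user's health ratio is below full before pickup is allowed.
; On pickup, it applies its restore amount through the user's HealthComponent with a clamped health change.
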(event `self.BlueprintHandlePickup`
  (params (ForUser :type "GladiatorCharacter Object Reference"))
  (`HealthComponent.ModifyHealthClamped` (`GladiatorCharacter.HealthComponent` ForUser) (`self.AmountToRestore`)))

(fn `BlueprintCanPickup`
  (params (ForUser :type "GladiatorCharacter Object Reference"))
  (returns (ReturnValue :type Boolean))
  (bind _returnvalue (`parent.BlueprintCanPickup` ForUser))
  (return (and _returnvalue (< (`HealthComponent.GetHealthRatio` (`GladiatorCharacter.HealthComponent` ForUser)) 1.0))))

(fn `UserConstructionScript`
  (`parent.UserConstructionScript`))