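; GA_ShrapnelShot is a Gameplay Ability that drives the Super Shotty weapon's shrapnel shot while the input is held.
; On activation it starts firing on the avatar's currently equipped BP_SuperShotty, ending at once if the avatar or weapon cast fails.
; On input release it calls EndFire on that ShrapnelShot and ends the ability, delegating the actual firing logic to the weapon.
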(event `self.K2_ActivateAbility`
  (`AbilityTask_WaitInputRelease.WaitInputRelease` false
    (:`then`
      (bind _asgladiator_character (cast `GladiatorCharacter` (`self.GetAvatarActorFromActorInfo`))
        (:`then`
          (bind _asbp_super_shotty (cast `/Game/Items/Weapons/BP_SuperShotty` (`GladiatorCharacter.CurrentEquipable` _asgladiator_character))
            (:`then`
              (`BulletFiringComponent.StartFire` (`/Game/Items/Weapons/BP_SuperShotty.ShrapnelShot` _asbp_super_shotty)))
            (:`CastFailed`
              (`self.K2_EndAbility` :!label _label))))
        (:`CastFailed`
          (goto _label))))
    (:`OnRelease`
      (bind _asgladiator_character_2 (cast `GladiatorCharacter` (`self.GetAvatarActorFromActorInfo`))
        (:`then`
          (bind _asbp_super_shotty_2 (cast `/Game/Items/Weapons/BP_SuperShotty` (`GladiatorCharacter.CurrentEquipable` _asgladiator_character_2))
            (:`then`
              (`BulletFiringComponent.EndFire` (`/Game/Items/Weapons/BP_SuperShotty.ShrapnelShot` _asbp_super_shotty_2)))
            (:`CastFailed`
              _)))
        (:`CastFailed`
          _))
      (`self.K2_EndAbility`))))