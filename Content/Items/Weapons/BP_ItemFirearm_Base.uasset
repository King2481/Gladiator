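; BP_ItemFirearm_Base is a base weapon item Blueprint for firearms.
; On BeginPlay it links its BulletFiring component to its AmmoComponent and to a mesh.
; That mesh is the first-person weapon mesh when the owner is a GladiatorCharacter, otherwise the item's own Mesh3P.
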(event `self.ReceiveBeginPlay`
  (set `BulletFiringComponent.LinkedAmmoComponent` (`self.AmmoComponent`) (`self.BulletFiring`))
  (bind _asgladiator_character (cast `GladiatorCharacter` (`self.GetOwner`))
    (:`then`
      (set `BulletFiringComponent.LinkedMeshComponent` (`GladiatorCharacter.WeaponMesh1P` _asgladiator_character) (`self.BulletFiring`)))
    (:`CastFailed`
      (set `BulletFiringComponent.LinkedMeshComponent` (`self.Mesh3P`) (`self.BulletFiring`)))))

(fn `UserConstructionScript`)