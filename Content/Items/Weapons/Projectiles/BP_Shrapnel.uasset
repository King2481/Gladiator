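; BP_Shrapnel is a shrapnel projectile that deals point damage to the first Character it hits.
; Its sphere collision hit event applies the damage with the shrapnel damage type along the reversed impact normal, then destroys the actor, both only on the server.
; Hits on anything else count as bounces, each renewing a short lifespan until the third, when the server destroys it.
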(event `self.SphereCollision.OnComponentHit`
  (params (HitComponent :type "PrimitiveComponent Object Reference") (OtherActor :type "Actor Object Reference") (OtherComp :type "PrimitiveComponent Object Reference") (NormalImpulse :type "Vector Structure") (Hit :type "HitResult Structure (by ref)"))
  (cast `Character` OtherActor
    (:`then`
      (`/Engine/EditorBlueprintResources/ActorMacros.Switch Has Authority`
        (:`Authority`
          (`GameplayStatics.ApplyPointDamage` OtherActor 25.0 (* (`.ImpactNormal` (`GameplayStatics.BreakHitResult` Hit)) -1.0) Hit (`self.GetInstigatorController`) self "/Game/Items/Weapons/DamageTypes/BP_DamageType_Shrapnel.BP_DamageType_Shrapnel_C")
          (`self.K2_DestroyActor` :!label _label))))
    (:`CastFailed`
      (bind _output_get (set `self.Number of Bounces` (+ (`self.Number of Bounces`) 1)))
      (if (>= _output_get 3)
        (`/Engine/EditorBlueprintResources/ActorMacros.Switch Has Authority`
          (:`Authority`
            (goto _label)))
        (else
          (`self.SetLifeSpan` 1.0) ; Keep giving it life
        )))))

(fn `UserConstructionScript`
  (`parent.UserConstructionScript`))