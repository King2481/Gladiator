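; BP_Projectile_Rivet is a rivet weapon projectile that damages characters and passes through them, with all gameplay logic running on the server.
; Sphere overlaps with Characters apply point damage using the riveter damage type, credited to the instigator's controller, and increment a penetration counter.
; The projectile destroys itself once that counter reaches its limit or when the collision sphere registers a blocking hit.
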(event `self.SphereCollision.OnComponentHit`
  (params (HitComponent :type "PrimitiveComponent Object Reference") (OtherActor :type "Actor Object Reference") (OtherComp :type "PrimitiveComponent Object Reference") (NormalImpulse :type "Vector Structure") (Hit :type "HitResult Structure (by ref)"))
  (`/Engine/EditorBlueprintResources/ActorMacros.Switch Has Authority`
    (:`Authority`
      (`self.K2_DestroyActor`))))

(event `self.SphereCollision.OnComponentBeginOverlap`
  (params (OverlappedComponent :type "PrimitiveComponent Object Reference") (OtherActor :type "Actor Object Reference") (OtherComp :type "PrimitiveComponent Object Reference") (OtherBodyIndex :type Integer) (bFromSweep :type Boolean) (SweepResult :type "HitResult Structure (by ref)"))
  (`/Engine/EditorBlueprintResources/ActorMacros.Switch Has Authority`
    (:`Authority`
      (bind _ascharacter (cast `Character` OtherActor))
      (`GameplayStatics.ApplyPointDamage` _ascharacter 50.0 (`.ImpactNormal` (`GameplayStatics.BreakHitResult` SweepResult)) SweepResult (`self.GetInstigatorController`) self "/Game/Items/Weapons/DamageTypes/BP_DamageType_Riviter.BP_DamageType_Riviter_C")
      (bind _output_get (set `self.TimesPenetrated` (+ (`self.TimesPenetrated`) 1)))
      (if (>= _output_get 5)
        (`self.K2_DestroyActor`)))))

(fn `UserConstructionScript`
  (`parent.UserConstructionScript`))