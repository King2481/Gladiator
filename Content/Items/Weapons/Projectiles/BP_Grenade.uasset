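; Grenade projectile that explodes when a five-second fuse runs out or when it hits a Character.
; On BeginPlay the mesh ignores its instigator when moving, then the server randomizes its rotation and starts the fuse timer.
; Timer expiry and server-side Character hits share one path that triggers the Explosion component and destroys the actor.
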(event `self.ReceiveBeginPlay`
  (`PrimitiveComponent.IgnoreActorWhenMoving` (`self.StaticMesh`) (`self.GetInstigator`) true)
  (`/Engine/EditorBlueprintResources/ActorMacros.Switch Has Authority`
    (:`Authority`
      (`SceneComponent.K2_SetWorldRotation` (`self.StaticMesh`) (`KismetMathLibrary.RandomRotator` true) false false)
      (bind _returnvalue (`KismetSystemLibrary.K2_SetTimerDelegate` (delegate `Explode`) 5.0))
      (set `self.ExplosionTimer` _returnvalue))))

(event `Explode`
  (`KismetSystemLibrary.K2_ClearAndInvalidateTimerHandle` (`self.ExplosionTimer`))
  (`ExplosionComponent.Explode` (`self.Explosion`) :!label _label)
  (`self.K2_DestroyActor`))

(event `self.StaticMesh.OnComponentHit`
  (params (HitComponent :type "PrimitiveComponent Object Reference") (OtherActor :type "Actor Object Reference") (OtherComp :type "PrimitiveComponent Object Reference") (NormalImpulse :type "Vector Structure") (Hit :type "HitResult Structure (by ref)"))
  (`/Engine/EditorBlueprintResources/ActorMacros.Switch Has Authority`
    (:`Authority`
      (cast `Character` OtherActor)
      (goto _label))))

(fn `UserConstructionScript`
  (`parent.UserConstructionScript`))