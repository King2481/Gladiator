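; Deathmatch game mode for gladiator matches that ends the round when a player reaches the kill target.
; On each character kill, it resolves the instigating controller's gladiator pawn and player state, then reads kills from that state's KillTrackingComponent.
; Reaching ScoreNeededToWin records that player state as the winner and switches the in-game state to RoundWon.
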(event `self.BlueprintOnCharacterKilled`
  (params (Victim :type "GladiatorCharacter Object Reference") (KillingDamage :type "Float (single-precision)") (DamageType :type "DamageType Object Reference") (EventInstigator :type "Controller Object Reference") (DamageCauser :type "Actor Object Reference"))
  (bind _asgladiator_character (cast `GladiatorCharacter` (`Controller.K2_GetPawn` EventInstigator)))
  (bind _asgladiator_player_state (cast `GladiatorPlayerState` (`Pawn.PlayerState` _asgladiator_character)))
  (bind _killtrackingcomponent (`GladiatorPlayerState.KillTrackingComponent` _asgladiator_player_state))
  (`/Engine/EditorBlueprintResources/StandardMacros.IsValid` _killtrackingcomponent
    (:`Is Valid`
      (bind _matchstats_kills (break `MatchStats` (`KillTrackingComponent.MatchStats` _killtrackingcomponent)))
      (if (>= _matchstats_kills (`self.ScoreNeededToWin`))
        (set `self.WinningPlayerState` _asgladiator_player_state)
        (`self.SetInGameState` "/Game/GameModes/InGameStates/RoundWon.RoundWon")))))

(fn `UserConstructionScript`
  (`parent.UserConstructionScript`))