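; BP_GameMode_TDM is a team-based game mode, apparently team deathmatch, that ends the round on a score limit.
; On each character kill event, it reads the Gladiator game state and compares the first team's score to ScoreNeededToWin.
; On reaching the limit, it records that team as winner and sets the RoundWon state.
; Only team 0 is checked; the graph has no win check for other teams.
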(event `self.BlueprintOnCharacterKilled`
  (params (Victim :type "GladiatorCharacter Object Reference") (KillingDamage :type "Float (single-precision)") (DamageType :type "DamageType Object Reference") (EventInstigator :type "Controller Object Reference") (DamageCauser :type "Actor Object Reference"))
  (bind _asgladiator_game_state (cast `GladiatorGameState` (`GameplayStatics.GetGameState`)))
  (bind _output (`|GetArrayItem` (`GladiatorGameState.Teams` _asgladiator_game_state)))
  (`/Engine/EditorBlueprintResources/StandardMacros.IsValid` _output
    (:`Is Valid`
      (if (>= (`TeamInfo.TeamScore` _output) (`self.ScoreNeededToWin`))
        (set `self.WinningTeamId` 0)
        (`self.SetInGameState` "/Game/GameModes/InGameStates/RoundWon.RoundWon")))))

(fn `UserConstructionScript`
  (`parent.UserConstructionScript`))